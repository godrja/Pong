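; Game mode Blueprint for a Pong game that handles the round reset when the ball goes out.
; On BeginPlay it finds the Ball actor and binds to its OnBallOut event.
; Each out event relaunches the ball with a direction chosen from the reported player, intended to throw toward the opposite side, then resets the position of every Paddle in the level.
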(event Custom|On%20Ball%20Out
  (params (player :type EPlayer%20Enum))
  (Utilities|HandleBallOutEvent player))

(event EventBeginPlay
  (bind _outactors (Actor|GetAllActorsOfClass "/Script/Pong.Ball"))
  (bind _output_get (Variables|Default|SetThe%20Ball (Utilities|Array|Get(acopy) _outactors)))
  (EventDispatchers|AssignOnBallOut _output_get (delegate Custom|On%20Ball%20Out)))

(fn ConstructionScript)

(fn ResetPaddles
  ;[1 1 1] Reset position of all paddles
  (bind _outactors (Actor|GetAllActorsOfClass "/Script/Pong.Paddle"))
  (for _array_element _outactors
    (Class|Paddle|ResetPosition _array_element)))
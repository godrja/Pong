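; Game state for a Pong game that keeps the left and right players' scores.
; On BeginPlay it finds the first Ball actor in the level and binds to its OnBallOut event.
; Each ball-out event increments the score of the player it passes, and two getter functions expose the left and right scores.
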(event Custom|Event%20BallOut
  (params (player :type EPlayer%20Enum))
  (switch Utilities|FlowControl|Switch|SwitchonEPlayer player
    (:P_RIGHT
      (bind _result (Math|Integer|IncrementInt (Variables|Score|GetRight%20Score))
        (:%20%20
          (Variables|Score|SetRight%20Score _result))))
    (:P_LEFT
      (bind _result_2 (Math|Integer|IncrementInt (Variables|Score|GetLeft%20Score))
        (:%20%20
          (Variables|Score|SetLeft%20Score _result_2))))))

(event EventBeginPlay
  (bind _outactors (Actor|GetAllActorsOfClass "/Script/Pong.Ball"))
  (EventDispatchers|BindEventtoOnBallOut (Utilities|Array|Get(acopy) _outactors) (delegate Custom|Event%20BallOut)))

(fn ConstructionScript)

(fn GetLeftScore
  (return (Variables|Score|GetLeft%20Score)))

(fn GetRightScore
  (return (Variables|Score|GetRight%20Score)))
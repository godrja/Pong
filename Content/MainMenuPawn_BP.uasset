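; Pawn for the main menu that owns the MainMenu_BP widget and drives it from player input.
; It creates the widget on BeginPlay, moves the selection with up and down actions, and on select either starts the game or quits.
; Any key press while paused triggers a game reset.
; Display and hide functions add or remove the widget, optionally switching the view to a supplied camera.
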(event EventBeginPlay
  (bind _returnvalue (UserInterface|CreateWidget "/Game/GUI/MainMenu_BP.MainMenu_BP_C" (Game|GetPlayerController 0)))
  (Variables|Default|SetMain%20Menu _returnvalue))

(event Input|ActionEvents|InputActionMenuUp
  (params (Key :type Key%20Structure :default "AnyKey"))
  (:Pressed
    (Default|MenuGoUp (Variables|Default|GetMain%20Menu))))

(event Input|ActionEvents|InputActionMenuDown
  (params (Key :type Key%20Structure :default "AnyKey"))
  (:Pressed
    (Default|MenuGoDown (Variables|Default|GetMain%20Menu))))

(event Input|ActionEvents|InputActionMenuSelect
  (params (Key :type Key%20Structure :default "AnyKey"))
  (:Pressed
    (switch Utilities|FlowControl|Switch|SwitchonMenuItem (Variables|/Game/GUI/MainMenu_BP.MainMenu_BP_C|GetSelected%20Item (Variables|Default|GetMain%20Menu))
      (:NewEnumerator0
        (Default|CallGameStart))
      (:NewEnumerator1
        (Game|QuitGame 0 "Quit")))))

(event Input|KeyboardEvents|AnyKey
  (params (Key :type Key%20Structure :default "AnyKey"))
  (:Pressed
    (if (Game|IsGamePaused)
      (Default|CallGameReset))))

(fn ConstructionScript)

(fn DisplayMenu
  (params (Custom%20Camera :type Camera%20Actor%20Object%20Reference))
  (UserInterface|Viewport|AddtoViewport (Variables|Default|GetMain%20Menu) 0)
  (Utilities|IsValid Custom%20Camera
    (:Is%20Valid
      (Game|Player|SetViewTargetwithBlend (Game|GetPlayerController 0) Custom%20Camera 0.0 "VTBlend_Linear" 0.0 false))))

(fn HideMenu
  (Widget|RemovefromParent (Variables|Default|GetMain%20Menu)))
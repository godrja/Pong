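; MyPawn_BP is a pawn Blueprint that turns player input into main menu navigation and selection.
; Menu Up and Menu Down actions move through the MainMenu object.
; Menu Select switches on its SelectedItem to either start the game or quit.
; An Any Key binding prints a debug string, and the construction script is empty.
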(event Input|ActionEvents|InputActionMenuUp
  (params (Key :type Key%20Structure :default "AnyKey"))
  (:Pressed
    (Default|MenuGoUp (Variables|Default|GetMain%20Menu))))

(event Input|ActionEvents|InputActionMenuDown
  (params (Key :type Key%20Structure :default "AnyKey"))
  (:Pressed
    (Default|MenuGoDown (Variables|Default|GetMain%20Menu))))

(event Input|ActionEvents|InputActionMenuSelect
  (params (Key :type Key%20Structure :default "AnyKey"))
  (:Pressed
    (switch Utilities|FlowControl|Switch|SwitchonMenuItem (Variables|/Game/GUI/MainMenu_BP.MainMenu_BP_C|GetSelected%20Item (Variables|Default|GetMain%20Menu))
      (:NewEnumerator0
        (Default|CallGameStart))
      (:NewEnumerator1
        (Game|QuitGame 0 "Quit")))))

(event Input|KeyboardEvents|AnyKey
  (params (Key :type Key%20Structure :default "AnyKey"))
  (:Pressed
    (Development|PrintString "Any Key Pressed")))

(fn ConstructionScript)
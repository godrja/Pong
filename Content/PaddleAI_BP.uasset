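; AI controller that drives a Paddle_BP pawn to follow the ball along the X axis.
; BeginPlay caches the first Ball_BP actor found in the level.
; Each tick it sets the paddle's CurrentSpeed to the signed X offset from paddle to ball, so speed scales with distance.
; A small dead zone zeroes the speed when the two are nearly aligned, which prevents jittering.
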(event EventBeginPlay
  ;[1 1 1] Get Reference to TheBall
  (bind _outactors (Actor|GetAllActorsOfClass "/Game/Ball_BP.Ball_BP_C"))
  (Variables|Default|SetTheBall (Utilities|Array|Get(acopy) _outactors)))

(event EventTick
  (params (DeltaSeconds :type Float%20%28single-precision%29))
  (bind _returnvalue (Pawn|GetControlledPawn))
  (bind _theball (Variables|Default|GetTheBall))
  (bind _returnvalue_2 (Transformation|GetActorLocation _returnvalue))
  (bind _returnvalue_3 (Transformation|GetActorLocation _theball))
  (bind _x (Math|Vector|BreakVector _returnvalue_2))
  (bind _x_2 (Math|Vector|BreakVector _returnvalue_3))
  (bind _returnvalue_4 (- _x_2 _x))
  ;[1 1 1] Move Paddle to the Ball
  (bind _aspaddle_bp (Utilities|Casting|CastToPaddle_BP _returnvalue))
  ;;[1 1 1] Fight Jittering
  (if (>= (Math|Float|Absolute(Float) _returnvalue_4) 1e+01)
    (Variables|/Game/Paddle_BP.Paddle_BP_C|SetCurrent%20Speed _aspaddle_bp _returnvalue_4)
    (else
      (Variables|/Game/Paddle_BP.Paddle_BP_C|SetCurrent%20Speed _aspaddle_bp 0.0))))

(fn ConstructionScript)